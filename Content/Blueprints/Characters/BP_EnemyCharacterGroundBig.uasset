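; BP_EnemyCharacterGroundBig is an enemy character Blueprint that drives an overhead health bar from its HealthComponent.
; On BeginPlay it caches the progress bar from the AI-Health widget.
; Each hurt event updates and shows the bar, which turns red and stays visible below one third health, and otherwise hides after two seconds.
; When health runs out, it hides the bar and resets its color to green.
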(event OnNoHealth(HealthComponent)
  (params (NewHealth :type Float%20%28single-precision%29))
  ;[0.1172 0.08438 0.15 0.5] Handle Health Bar
  (Rendering|SetVisibility (Variables|Default|GetHealthBar) false false)
  (Class|ProgressBar|SetFillColorandOpacity (Variables|Default|GetHealth%20Progress%20Bar) "(R=0.333333,G=1.000000,B=0.000000,A=0.500000)"))

(event OnHurt(HealthComponent)
  (params (NewHealth :type Float%20%28single-precision%29))
  (bind _healthcomponent (Variables|Default|GetHealthComponent))
  (bind _returnvalue (Class|SGHealthComponent|GetMaxHealth _healthcomponent))
  ;[0.1172 0.08438 0.15 0.5] Handle Health Bar
  (Progress|SetPercent (Variables|Default|GetHealth%20Progress%20Bar) (/ NewHealth _returnvalue))
  (Rendering|SetVisibility (Variables|Default|GetHealthBar) true false)
  (if (< NewHealth (/ _returnvalue 3.0))
    (Class|ProgressBar|SetFillColorandOpacity (Variables|Default|GetHealth%20Progress%20Bar) "(R=1.000000,G=0.000000,B=0.000000,A=0.500000)")
    (else
      (Utilities|FlowControl|Delay 2.0)
      (Rendering|SetVisibility (Variables|Default|GetHealthBar) false false))))

(event EventBeginPlay
  ;[0.15 0.15 0.15 0.5] Set Health Bar
  (bind _asai_health (Utilities|Casting|CastToAI-Health (UserInterface|GetWidget (Variables|Default|GetHealthBar))))
  (Variables|Default|SetHealth%20Progress%20Bar (Variables|/Game/Blueprints/AI/VFX/AI-Health.AI-Health_C|GetHealthBar _asai_health)))

(fn ConstructionScript)