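; Player character Blueprint that handles first-level weapon animation for a rifle, shotgun and grenade launcher.
; BPFire, BPReload and BPWeaponSwap events play montages on WeaponMesh.
; Swaps set exclusive weapon bools on WeaponAnimBP, which BPFire reads to pick the shoot montage; BeginPlay defaults to rifle.
; Input events are empty, while game-over, damage-effect, fire-rate calculation and ammo-check logic are left unconnected.
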(event Input|EnhancedActionEvents|EnhancedInputActionIA_SwapWeapon2
  (params (ActionValue :type Boolean) (ElapsedSeconds :type Float%20%28double-precision%29) (TriggeredSeconds :type Float%20%28double-precision%29) (InputAction :type Input%20Action%20Object%20Reference :default "/Game/Input/InputActions/IA_SwapWeapon2.IA_SwapWeapon2")))

(event Input|EnhancedActionEvents|EnhancedInputActionIA_SwapWeapon1
  (params (ActionValue :type Boolean) (ElapsedSeconds :type Float%20%28double-precision%29) (TriggeredSeconds :type Float%20%28double-precision%29) (InputAction :type Input%20Action%20Object%20Reference :default "/Game/Input/InputActions/IA_SwapWeapon1.IA_SwapWeapon1")))

(event Input|EnhancedActionEvents|EnhancedInputActionIA_SwapWeapon3
  (params (ActionValue :type Boolean) (ElapsedSeconds :type Float%20%28double-precision%29) (TriggeredSeconds :type Float%20%28double-precision%29) (InputAction :type Input%20Action%20Object%20Reference :default "/Game/Input/InputActions/IA_SwapWeapon3.IA_SwapWeapon3")))

(event EventBeginPlay
  ;[0.15 0.15 0.15 0.5] Sätt en bool så vapnet kan börja idlea i AnimBP
  (bind _asweapon_anim_bp (Utilities|Casting|CastToWeaponAnimBP (Components|SkeletalMesh|GetAnimInstance (Variables|Default|GetWeaponMesh))))
  (Variables|/Game/Weapon/Gun/WeaponAnimBP.WeaponAnimBP_C|SetRifle _asweapon_anim_bp true)
  (Variables|/Game/Weapon/Gun/WeaponAnimBP.WeaponAnimBP_C|SetShotgun _asweapon_anim_bp false)
  (Variables|/Game/Weapon/Gun/WeaponAnimBP.WeaponAnimBP_C|SetGrenade_Launcher _asweapon_anim_bp false))

(event Collision|EventActorBeginOverlap
  (params (OtherActor :type Actor%20Object%20Reference)))

(event EventTick
  (params (DeltaSeconds :type Float%20%28single-precision%29)))

(event EventBPWeaponSwapAR
  ;[0.15 0.15 0.15 0.5] Byt till Rifle
  (Animation|Montage|PlayMontage (Variables|Default|GetWeaponMesh) "/Game/Weapon/Gun/AM_Rifle_in.AM_Rifle_in"
    (:then
      (bind _asweapon_anim_bp (Utilities|Casting|CastToWeaponAnimBP (Components|SkeletalMesh|GetAnimInstance (Variables|Default|GetWeaponMesh))))
      (Variables|/Game/Weapon/Gun/WeaponAnimBP.WeaponAnimBP_C|SetRifle _asweapon_anim_bp true)
      (Variables|/Game/Weapon/Gun/WeaponAnimBP.WeaponAnimBP_C|SetShotgun _asweapon_anim_bp false)
      (Variables|/Game/Weapon/Gun/WeaponAnimBP.WeaponAnimBP_C|SetGrenade_Launcher _asweapon_anim_bp false))))

(event EventBPReload
  ;[0.15 0.15 0.15 0.5] Reload Rifle
  (Animation|Montage|PlayMontage (Variables|Default|GetWeaponMesh) "/Game/Weapon/Gun/AM_Reload.AM_Reload"))

(event EventBPWeaponSwapGL
  ;[0.15 0.15 0.15 0.5] Byt till Grenade Launcher
  (Animation|Montage|PlayMontage (Variables|Default|GetWeaponMesh) "/Game/Weapon/Gun/AM_Grenade_in.AM_Grenade_in"
    (:then
      (bind _asweapon_anim_bp (Utilities|Casting|CastToWeaponAnimBP (Components|SkeletalMesh|GetAnimInstance (Variables|Default|GetWeaponMesh))))
      (Variables|/Game/Weapon/Gun/WeaponAnimBP.WeaponAnimBP_C|SetGrenade_Launcher _asweapon_anim_bp true)
      (Variables|/Game/Weapon/Gun/WeaponAnimBP.WeaponAnimBP_C|SetRifle _asweapon_anim_bp false)
      (Variables|/Game/Weapon/Gun/WeaponAnimBP.WeaponAnimBP_C|SetShotgun _asweapon_anim_bp false))))

(event EventBPWeaponSwapSG
  ;[0.15 0.15 0.15 0.5] Byt till Shotgun
  (Animation|Montage|PlayMontage (Variables|Default|GetWeaponMesh) "/Game/Weapon/Gun/AM_Shotgun_in.AM_Shotgun_in"
    (:then
      (bind _asweapon_anim_bp (Utilities|Casting|CastToWeaponAnimBP (Components|SkeletalMesh|GetAnimInstance (Variables|Default|GetWeaponMesh))))
      (Variables|/Game/Weapon/Gun/WeaponAnimBP.WeaponAnimBP_C|SetShotgun _asweapon_anim_bp true)
      (Variables|/Game/Weapon/Gun/WeaponAnimBP.WeaponAnimBP_C|SetRifle _asweapon_anim_bp false)
      (Variables|/Game/Weapon/Gun/WeaponAnimBP.WeaponAnimBP_C|SetGrenade_Launcher _asweapon_anim_bp false)
      (Development|PrintString "Shotgun in"))))

(event EventBPFire
  ;[0.15 0.15 0.15 0.5] Skjut & casta
  (bind _asweapon_anim_bp (Utilities|Casting|CastToWeaponAnimBP (Components|SkeletalMesh|GetAnimInstance (Variables|Default|GetWeaponMesh))))
  ;[0.15 0.15 0.15 0.5] Skjut animation triggas baserat på bool
  (if (Variables|/Game/Weapon/Gun/WeaponAnimBP.WeaponAnimBP_C|GetRifle _asweapon_anim_bp)
    (if true
      (Animation|Montage|PlayMontage (Variables|Default|GetWeaponMesh) "/Game/Weapon/Gun/AM_Rifle_shoot_mont.AM_Rifle_shoot_mont" (Utilities|Firerate)))
    (elif (Variables|/Game/Weapon/Gun/WeaponAnimBP.WeaponAnimBP_C|GetShotgun _asweapon_anim_bp)
      (Animation|Montage|PlayMontage (Variables|Default|GetWeaponMesh) "/Game/Weapon/Gun/AM_Shotgun_shoot.AM_Shotgun_shoot")
      (else
        (Animation|Montage|PlayMontage (Variables|Default|GetWeaponMesh) "/Game/Weapon/Gun/AM_Grenade_shoot.AM_Grenade_shoot")))))

(fn ConstructionScript)