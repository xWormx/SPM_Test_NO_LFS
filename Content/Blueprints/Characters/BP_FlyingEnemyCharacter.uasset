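; BP_FlyingEnemyCharacter is the Blueprint for a flying enemy character, and its graph drives the enemy's health bar.
; BeginPlay casts the HealthBar component's widget to WBP_EnemyHealthBar and caches its progress bar.
; HealthComponent's OnHurt and OnNoHealth events pass the bar to shared HandleDeathBar functions, with current and maximum health supplied on hurt.
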(event OnNoHealth(HealthComponent)
  (params (NewHealth :type Float%20%28single-precision%29))
  ;[0.1172 0.08438 0.15 0.5] Handle Health Bar
  (Class|SGEnemyCharacter|HandleDeathBaronDeath (Variables|Default|GetHealthBar) (Variables|Default|GetHealth%20Progress%20Bar)))

(event OnHurt(HealthComponent)
  (params (NewHealth :type Float%20%28single-precision%29))
  ;[0.1172 0.08438 0.15 0.5] Handle Health Bar
  (Class|SGEnemyCharacter|HandleDeathBaronHurt NewHealth (Class|SGHealthComponent|GetMaxHealth (Variables|Default|GetHealthComponent)) (Variables|Default|GetHealthBar) (Variables|Default|GetHealth%20Progress%20Bar)))

(event EventBeginPlay
  ;[0.15 0.15 0.15 0.5] Set Health Bar
  (bind _asai_health (Utilities|Casting|CastToWBP_EnemyHealthBar (UserInterface|GetWidget (Variables|Default|GetHealthBar))))
  (Variables|Default|SetHealth%20Progress%20Bar (Variables|/Game/Blueprints/AI/VFX/WBP_EnemyHealthBar.WBP_EnemyHealthBar_C|GetHealthBar _asai_health)))

(fn ConstructionScript)