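; Secret heart pickup that beats in the world and reskins the player's weapon when touched.
; A self-rescheduling one-second timer event runs the HeartBeat macro, which chains two delayed Pulse scale bumps into a double thump.
; Any overlap with the sphere hides the mesh, disables its collision and applies the alternate gun material to the weapon mesh of the player cached at BeginPlay.
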(event OnComponentBeginOverlap(Sphere)
  (params (OverlappedComponent :type Primitive%20Component%20Object%20Reference) (OtherActor :type Actor%20Object%20Reference) (OtherComp :type Primitive%20Component%20Object%20Reference) (OtherBodyIndex :type Integer) (bFromSweep :type Boolean) (SweepResult :type Hit%20Result%20Structure%20%28by%20ref%29))
  (bind _staticmeshcomponent (Variables|Debug|GetStaticMeshComponent))
  (Development|SetHiddeninGame _staticmeshcomponent true false)
  (Collision|SetCollisionEnabled _staticmeshcomponent "NoCollision")
  (Rendering|Material|SetMaterial (Variables|/Script/SPM_Test_NO_LFS.SGPlayerCharacter|GetWeaponMesh (Variables|Default|GetPlayer)) 4 "/Game/Weapon/Material/HugosGun/M_Altgun.M_Altgun"))

(event Custom|Dun-Dun
  (Utilities|HeartBeat)
  (Utilities|Time|SetTimerbyFunctionName 0 "Dun-Dun" 1.0))

(event EventBeginPlay
  (bind _asbp_sgplayer_character (Utilities|Casting|CastToBP_SGPlayerCharacter (Game|GetPlayerCharacter 0)))
  (Variables|Default|SetPlayer _asbp_sgplayer_character)
  (CallFunction|Dun-Dun))

(fn ConstructionScript)