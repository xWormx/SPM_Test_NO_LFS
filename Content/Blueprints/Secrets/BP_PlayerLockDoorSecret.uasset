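; BP_PlayerLockDoorSecret is a secret door that opens once both of its keys are activated, in either order.
; Overlapping either key sphere hides that key, reveals its counterpart mesh (Key3 or Key4) and sets that key's flag.
; When both flags are set, the static mesh is hidden and its collision disabled.
; The overlap events do not check which actor triggers them.
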(event OnComponentBeginOverlap(Key1Sphere)
  (params (OverlappedComponent :type Primitive%20Component%20Object%20Reference) (OtherActor :type Actor%20Object%20Reference) (OtherComp :type Primitive%20Component%20Object%20Reference) (OtherBodyIndex :type Integer) (bFromSweep :type Boolean) (SweepResult :type Hit%20Result%20Structure%20%28by%20ref%29))
  (Development|SetHiddeninGame (Variables|Default|Getkey3) false false)
  (Development|SetHiddeninGame (Variables|Default|Getkey1) true false)
  (Variables|Default|Setkey1activated true)
  (if (Variables|Default|Getkey2activated)
    (Development|SetHiddeninGame (Variables|Debug|GetStaticMeshComponent) true false)
    (Collision|SetCollisionEnabled (Variables|Debug|GetStaticMeshComponent) "NoCollision")))

(event OnComponentBeginOverlap(Key2Sphere)
  (params (OverlappedComponent :type Primitive%20Component%20Object%20Reference) (OtherActor :type Actor%20Object%20Reference) (OtherComp :type Primitive%20Component%20Object%20Reference) (OtherBodyIndex :type Integer) (bFromSweep :type Boolean) (SweepResult :type Hit%20Result%20Structure%20%28by%20ref%29))
  (Development|SetHiddeninGame (Variables|Default|Getkey4) false false)
  (Development|SetHiddeninGame (Variables|Default|Getkey2) true false)
  (Variables|Default|Setkey2activated true)
  (if (Variables|Default|Getkey1activated)
    (Development|SetHiddeninGame (Variables|Debug|GetStaticMeshComponent) true false)
    (Collision|SetCollisionEnabled (Variables|Debug|GetStaticMeshComponent) "NoCollision")))

(fn ConstructionScript)